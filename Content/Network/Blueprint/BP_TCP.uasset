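; BP_TCP is a TCP client that connects to a local server on BeginPlay and sends messages and user names, apparently for chat.
; Connection callbacks track the socket ID in ServerSocket.
; TCPSendMessage and TCPUserName both send raw bytes, calling the disconnect handler on failure, then setting ServerSocket to 0.
; The receive handler is empty; nodes for printing incoming text to the chat UI are unwired.
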(event Custom|TCPDisconnected
  (params (ConnectionId :type Integer))
  (Variables|Default|SetServerSocket -1))

(event Custom|TCPConnected
  (params (ConnectionId :type Integer))
  (Variables|Default|SetServerSocket ConnectionId))

(event Custom|OnRecvMessage
  (params (ConnectionId :type Integer) (Message :type Array%20of%20Bytes)))

(event EventBeginPlay
  (Class|TcpSocketConnection|Connect "127.0.0.1" 4949 (delegate Custom|TCPDisconnected) (delegate Custom|TCPConnected) (delegate Custom|OnRecvMessage)))

(fn ConstructionScript)

(fn TCPSendMessage
  (params (Message :type String))
  (bind _returnvalue (Class|TcpSocketConnection|SendData (Variables|Default|GetServerSocket) (Class|TcpSocketConnection|ToBytes(String) Message)))
  (if (not _returnvalue)
    (CallFunction|TCPDisconnected (Variables|Default|GetServerSocket))
    (Variables|Default|SetServerSocket 0)))

(fn TCPUserName
  (params (UserName :type String))
  (bind _returnvalue (Class|TcpSocketConnection|SendData (Variables|Default|GetServerSocket) (Class|TcpSocketConnection|ToBytes(String) UserName)))
  (if (not _returnvalue)
    (CallFunction|TCPDisconnected (Variables|Default|GetServerSocket))
    (Variables|Default|SetServerSocket 0)))