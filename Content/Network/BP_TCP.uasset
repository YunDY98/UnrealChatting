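; BP_TCP is a TCP client for chat that connects to a hardcoded localhost server on BeginPlay.
; It stores the connection ID in ServerSocket, resetting it on disconnect or failed send.
; Received messages are decoded to strings and printed through the player character's chat widget.
; TCPSendMessage sends text as bytes, printing a Korean success message or invoking the disconnect handler on failure.
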(event Custom|TCPDisconnected
  (params (ConnectionId :type Integer))
  (Variables|Default|SetServerSocket -1))

(event Custom|TCPConnected
  (params (ConnectionId :type Integer))
  (Variables|Default|SetServerSocket ConnectionId))

(event Custom|OnRecvMessage
  (params (ConnectionId :type Integer) (Message :type Array%20of%20Bytes))
  (bind _returnvalue (Class|TcpSocketConnection|MessageReadString Message (Utilities|Array|Length Message)))
  (bind _asthird_person_character (Utilities|Casting|CastToThirdPersonCharacter (Game|GetPlayerCharacter 0)))
  (Default|PrintRecvMessage (Variables|/Game/ThirdPersonBP/Blueprints/ThirdPersonCharacter.ThirdPersonCharacter_C|GetUMGChattingRef _asthird_person_character) _returnvalue))

(event EventBeginPlay
  (Class|TcpSocketConnection|Connect "127.0.0.1" 4949 (delegate Custom|TCPDisconnected) (delegate Custom|TCPConnected) (delegate Custom|OnRecvMessage)))

(fn ConstructionScript)

(fn TCPSendMessage
  (params (Message :type String))
  (bind _returnvalue (Class|TcpSocketConnection|SendData (Variables|Default|GetServerSocket) (Class|TcpSocketConnection|ToBytes(String) Message)))
  (if _returnvalue
    (Development|PrintString (Utilities|String|Append "메시지 전송성공 ! 메시지 : " Message))
    (else
      (CallFunction|TCPDisconnected (Variables|Default|GetServerSocket))
      (Variables|Default|SetServerSocket 0))))