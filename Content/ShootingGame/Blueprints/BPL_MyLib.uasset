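; BPL_MyLib is a small function library for validating text input in the shooting game.
; MyLibCheckTextLite passes text that is shorter than eight characters and in which a substring search, whose search literal appears empty, finds no match.
; MyLibCheckText is the stricter variant, adding a non-empty requirement on top of the Lite check.
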(fn MyLibCheckText
  (params (InputPin :type Text%20%28by%20ref%29))
  (return (and (Utilities|Enum|NotEqual(Enum) InputPin (Utilities|Text|MakeLiteralText "")) (CallFunction|MyLibCheckTextLite InputPin))))

(fn MyLibCheckTextLite
  (params (InputPin :type Text%20%28by%20ref%29))
  (bind _returnvalue (Utilities|String|ToString(Text) InputPin))
  (return (and (< (Utilities|String|Len _returnvalue) 8) (== (Utilities|String|FindSubstring _returnvalue " ") -1))))