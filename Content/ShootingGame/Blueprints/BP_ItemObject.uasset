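; BP_ItemObject is a world item pickup that an overlapping actor collects into its inventory.
; On BeginPlay it looks up its ItemRowName in DT_Item, stores the row and applies that row's static mesh if valid.
; When the mesh begins an overlap, it passes the row name to GetItem on the other actor's BP_InvenComponent and destroys itself if that returns true.
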(event OnComponentBeginOverlap(StaticMesh)
  (params (OverlappedComponent :type Primitive%20Component%20Object%20Reference) (OtherActor :type Actor%20Object%20Reference) (OtherComp :type Primitive%20Component%20Object%20Reference) (OtherBodyIndex :type Integer) (bFromSweep :type Boolean) (SweepResult :type Hit%20Result%20Structure%20%28by%20ref%29))
  (bind _success (Default|GetItem (Actor|GetComponentbyClass OtherActor "/Game/ShootingGame/Data/BP_InvenComponent.BP_InvenComponent_C") (Variables|Default|GetItemRowName)))
  (if _success
    (Actor|DestroyActor)))

(event EventBeginPlay
  (bind _returnvalue (Utilities|GetDataTableRow "/Game/ShootingGame/Data/DT_Item.DT_Item" (Variables|Default|GetItemRowName))
    (:then
      (bind _output_get (Variables|Default|SetItem _returnvalue))
      (Utilities|IsValid (.staticmesh _output_get)
        (:Is%20Valid
          (Components|StaticMesh|SetStaticMesh (Variables|Default|GetStaticMesh) (.staticmesh _output_get)))))))

(fn ConstructionScript)